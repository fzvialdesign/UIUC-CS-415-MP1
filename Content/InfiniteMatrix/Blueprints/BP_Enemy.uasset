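; BP_Enemy is an enemy actor that randomizes its Y and Z position on spawn and reacts to overlaps.
; Overlapping BP_Player calls its ProcessHit and destroys the enemy.
; Overlapping BP_Projectile updates the player's score and kill count through GetActorOfClass, then destroys the enemy.
; Any TriggerZone overlap destroys the first BP_Enemy that GetActorOfClass returns, which is not necessarily this instance.
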(event `self.ReceiveBeginPlay`
  (`self.K2_AddActorLocalOffset` (`KismetMathLibrary.MakeVector` 0.0 (`KismetMathLibrary.RandomFloatInRange` -300.0 300.0) (`KismetMathLibrary.RandomFloatInRange` -300.0 300.0))))

(event `self.ReceiveActorBeginOverlap`
  (params (OtherActor :type "Actor Object Reference"))
  (`|ExecutionSequence`
    (:`then_0`
      (bind _asbp_player (cast `/Game/InfiniteMatrix/Blueprints/BP_Player` OtherActor))
      (`/Game/InfiniteMatrix/Blueprints/BP_Player.ProcessHit` _asbp_player))
    (:`then_1`
      (cast `/Game/InfiniteMatrix/Blueprints/BP_Projectile` OtherActor)
      (bind _returnvalue (`GameplayStatics.GetActorOfClass` "/Game/InfiniteMatrix/Blueprints/BP_Player.BP_Player_C"))
      (`/Game/InfiniteMatrix/Blueprints/BP_Player.UpdateScore` _returnvalue)
      (`/Engine/EditorBlueprintResources/StandardMacros.IncrementInt` (`/Game/InfiniteMatrix/Blueprints/BP_Player.Kills` _returnvalue)
        (:`  `
          _))))
  (`self.K2_DestroyActor`))

(event `self.TriggerZone.OnComponentBeginOverlap`
  (params (OverlappedComponent :type "PrimitiveComponent Object Reference") (OtherActor :type "Actor Object Reference") (OtherComp :type "PrimitiveComponent Object Reference") (OtherBodyIndex :type Integer) (bFromSweep :type Boolean) (SweepResult :type "HitResult Structure (by ref)"))
  (bind _returnvalue (`GameplayStatics.GetActorOfClass` "BP_Enemy_C"))
  (`self.K2_DestroyActor` _returnvalue))

(fn `UserConstructionScript`)